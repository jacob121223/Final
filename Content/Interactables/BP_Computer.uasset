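; BP_Computer is an interactable computer that opens the way by destroying its TargetGate when the player has a disk.
; Overlapping its Box casts the actor to BP_PlayerCharacter, checks HasDisk and prints that value on screen in either case.
; The InteractWithComputer event only casts the player character, as its disk check and "Door is open!!" message are disconnected.
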(event OnComponentBeginOverlap(Box)
  (params (OverlappedComponent :type Primitive%20Component%20Object%20Reference) (OtherActor :type Actor%20Object%20Reference) (OtherComp :type Primitive%20Component%20Object%20Reference) (OtherBodyIndex :type Integer) (bFromSweep :type Boolean) (SweepResult :type Hit%20Result%20Structure%20%28by%20ref%29))
  (bind _asbp_player_character (Utilities|Casting|CastToBP_PlayerCharacter OtherActor))
  (if (Variables|/Game/Player/BP_PlayerCharacter.BP_PlayerCharacter_C|GetHasDisk _asbp_player_character)
    (Development|PrintString (Utilities|String|ToString(Boolean) (Variables|/Game/Player/BP_PlayerCharacter.BP_PlayerCharacter_C|GetHasDisk _asbp_player_character)) true true "(R=0.000000,G=0.660000,B=1.000000,A=1.000000)" 6e+01)
    (Actor|DestroyActor (Variables|Default|GetTargetGate))
    (else
      (Development|PrintString (Utilities|String|ToString(Boolean) (Variables|/Game/Player/BP_PlayerCharacter.BP_PlayerCharacter_C|GetHasDisk _asbp_player_character)) true true "(R=0.000000,G=0.660000,B=1.000000,A=1.000000)" 6e+01))))

(event Custom|InteractWithComputer
  (bind _asbp_player_character (Utilities|Casting|CastToBP_PlayerCharacter (Game|GetPlayerCharacter 0))))

(event Input|EnhancedActionEvents|EnhancedInputActionInput_Interact
  (params (ActionValue :type Boolean) (ElapsedSeconds :type Float%20%28double-precision%29) (TriggeredSeconds :type Float%20%28double-precision%29) (InputAction :type Input%20Action%20Object%20Reference :default "/Game/Inputs/Input_Interact.Input_Interact")))

(event EventBeginPlay)

(event Collision|EventActorBeginOverlap
  (params (OtherActor :type Actor%20Object%20Reference)))

(event EventTick
  (params (DeltaSeconds :type Float%20%28single-precision%29)))

(fn ConstructionScript)
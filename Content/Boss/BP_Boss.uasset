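; BP_Boss is a boss actor that takes damage until it is defeated.
; AnyDamage records the damage causer, subtracts the damage from Health and calls the CheckHealth custom event.
; CheckHealth prints the current health as on-screen debug text, then destroys the actor and prints a defeat message once Health reaches zero or below.
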(event Custom|CheckHealth
  (Development|PrintString "Boss" true true "(R=0.000000,G=0.660000,B=1.000000,A=1.000000)" 1e+02)
  (Development|PrintString (Utilities|String|ToString(Integer) (Variables|Default|GetHealth)) true true "(R=0.000000,G=0.660000,B=1.000000,A=1.000000)" 1e+02)
  (if (<= (Variables|Default|GetHealth) 0)
    (Actor|DestroyActor)
    (Development|PrintString "You Defeted the Boss!" true true "(R=0.000000,G=0.660000,B=1.000000,A=1.000000)" 1e+02)))

(event EventBeginPlay)

(event Collision|EventActorBeginOverlap
  (params (OtherActor :type Actor%20Object%20Reference)))

(event EventTick
  (params (DeltaSeconds :type Float%20%28single-precision%29)))

(event Game|Damage|EventAnyDamage
  (params (Damage :type Float%20%28single-precision%29) (DamageType :type Damage%20Type%20Object%20Reference) (InstigatedBy :type Controller%20Object%20Reference) (DamageCauser :type Actor%20Object%20Reference))
  (Variables|Default|SetDamageCauser DamageCauser)
  (Variables|Default|SetHealth (- (Variables|Default|GetHealth) Damage))
  (CallFunction|CheckHealth))

(fn ConstructionScript)
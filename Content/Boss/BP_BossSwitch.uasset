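; BP_BossSwitch is a one-shot switch that damages an assigned Boss when the player triggers it from above.
; Box overlap casts to BP_PlayerCharacter and requires the player to be sufficiently higher than the switch.
; It then sets Activated, disables Box collision and plays the Alpha timeline, whose Finished output repositions Button and applies damage to Boss.
; An already activated switch only prints a debug string.
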(event OnComponentBeginOverlap(Box)
  (params (OverlappedComponent :type Primitive%20Component%20Object%20Reference) (OtherActor :type Actor%20Object%20Reference) (OtherComp :type Primitive%20Component%20Object%20Reference) (OtherBodyIndex :type Integer) (bFromSweep :type Boolean) (SweepResult :type Hit%20Result%20Structure%20%28by%20ref%29))
  (bind _asbp_player_character (Utilities|Casting|CastToBP_PlayerCharacter OtherActor))
  (if (> (.z (Transformation|GetActorLocation _asbp_player_character)) (+ (.z (Transformation|GetActorLocation)) 8e+01))
    (if (Variables|Default|GetActivated)
      (Development|PrintString (Utilities|String|ToString(Boolean) (Variables|Default|GetActivated)) true true "(R=1.000000,G=1.000000,B=1.000000,A=1.000000)" 1e+02)
      (else
        (Variables|Default|SetActivated true)
        (Collision|SetCollisionEnabled (Variables|Default|GetBox) "NoCollision")
        (Timeline|Alpha Play
          (:Finished
            (Transformation|SetRelativeLocation (Variables|Default|GetButton) "0.000000,0.000000,2.000000" false false)
            (Game|Damage|ApplyDamage (Variables|Default|GetBoss) 2e+01 0 0)))))))

(event EventBeginPlay)

(event Collision|EventActorBeginOverlap
  (params (OtherActor :type Actor%20Object%20Reference)))

(event EventTick
  (params (DeltaSeconds :type Float%20%28single-precision%29)))

(fn ConstructionScript)
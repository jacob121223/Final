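; Player character Blueprint handling movement, jumping and health, with turret projectiles as the intended damage source.
; Enhanced Input drives strafing and jumping, though forward input has a zero direction and Ongoing calls StopJumping.
; Projectile overlaps call ApplyDamage without a target; AnyDamage reduces Health and prints it, or at zero opens level "None" with a death message.
; Disk-gated door, level-load and death-message nodes remain unconnected.
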(event OnComponentBeginOverlap(CapsuleComponent)
  (params (OverlappedComponent :type Primitive%20Component%20Object%20Reference) (OtherActor :type Actor%20Object%20Reference) (OtherComp :type Primitive%20Component%20Object%20Reference) (OtherBodyIndex :type Integer) (bFromSweep :type Boolean) (SweepResult :type Hit%20Result%20Structure%20%28by%20ref%29))
  (bind _asbp_turret_proj (Utilities|Casting|CastToBP_TurretProj OtherActor))
  (Game|Damage|ApplyDamage 0 1e+01 0 _asbp_turret_proj))

(event Custom|CheckHealth
  (if (<= (Variables|Default|GetHealth) 0)
    (Game|OpenLevel(byName) "None")
    (Development|PrintString "You Died" true true "(R=0.000000,G=0.660000,B=1.000000,A=1.000000)" 3e+01)
    (else
      (Development|PrintString (Utilities|String|ToString(Integer) (Variables|Default|GetHealth)) true true "(R=0.000000,G=0.660000,B=1.000000,A=1.000000)" 3e+01))))

(event Input|EnhancedActionEvents|EnhancedInputActionInput_Movement
  (params (ActionValue :type Vector%202D%20Structure) (ElapsedSeconds :type Float%20%28double-precision%29) (TriggeredSeconds :type Float%20%28double-precision%29) (InputAction :type Input%20Action%20Object%20Reference :default "/Game/Inputs/Input_Movement.Input_Movement"))
  (bind _returnvalue (Pawn|GetControlRotation :!class /Script/Engine.Pawn))
  (Pawn|Input|AddMovementInput (Math|Vector|GetRightVector (Math|Rotator|MakeRotator (.roll _returnvalue) 0.0 (.yaw _returnvalue))) (.x ActionValue) false)
  (Pawn|Input|AddMovementInput "0, 0, 0" (.y ActionValue) false))

(event Input|EnhancedActionEvents|EnhancedInputActionInput_Jump
  (params (ActionValue :type Boolean) (ElapsedSeconds :type Float%20%28double-precision%29) (TriggeredSeconds :type Float%20%28double-precision%29) (InputAction :type Input%20Action%20Object%20Reference :default "/Game/Inputs/Input_Jump.Input_Jump"))
  (:Triggered
    (Character|Jump))
  (:Ongoing
    (Character|StopJumping)))

(event EventBeginPlay
  (bind _output_get (Variables|Default|SetHealth 100))
  (Development|PrintString (Utilities|String|ToString(Integer) _output_get)))

(event Collision|EventActorBeginOverlap
  (params (OtherActor :type Actor%20Object%20Reference)))

(event EventTick
  (params (DeltaSeconds :type Float%20%28single-precision%29)))

(event Game|Damage|EventAnyDamage
  (params (Damage :type Float%20%28single-precision%29) (DamageType :type Damage%20Type%20Object%20Reference) (InstigatedBy :type Controller%20Object%20Reference) (DamageCauser :type Actor%20Object%20Reference))
  (Variables|Default|SetDamageCauser DamageCauser)
  (Variables|Default|SetHealth (- (Variables|Default|GetHealth) Damage))
  (CallFunction|CheckHealth))

(fn ConstructionScript)